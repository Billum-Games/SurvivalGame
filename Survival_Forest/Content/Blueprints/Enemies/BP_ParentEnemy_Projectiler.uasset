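; Ranged enemy Blueprint that attacks the player with fireball projectiles.
; Its RangedAttack event casts the player character, turns the enemy to face it, then, if CanAttack is set, spawns BP_EnemyProjectile_Fireball at the SpawnProjectilePos transform.
; The enemy's minimum and maximum damage values are passed to each fireball on spawn.
; The construction script only calls the parent version.
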(event `/Game/Blueprints/Enemies/AI/Tasks/AttackInterface.RangedAttack`
  (bind _asthird_person_character (cast `/Game/ThirdPersonBP/Blueprints/ThirdPersonCharacter` (`GameplayStatics.GetPlayerCharacter` 0)))
  (`|ExecutionSequence`
    (:`then_0`
      (`self.K2_SetActorRelativeRotation` (`KismetMathLibrary.FindLookAtRotation` (`self.K2_GetActorLocation`) (`self.K2_GetActorLocation` _asthird_person_character))))
    (:`then_1`
      (if (`self.CanAttack`)
        (`|SpawnActorFromClass` "/Game/Blueprints/Enemies/BP_EnemyProjectile_Fireball.BP_EnemyProjectile_Fireball_C" (`SceneComponent.K2_GetComponentToWorld` (`self.SpawnProjectilePos`)) "Undefined" "OverrideRootScale" null (`self.DamageMin`) (`self.DamageMax`) null)))))

(fn `UserConstructionScript`
  (`parent.UserConstructionScript`))