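; Enemy fireball projectile actor, named as a soundless attack variant, that removes itself on impact or after a timeout.
; It adds an audio component on BeginPlay, and its box overlap destroys it on contact with anything except enemies, items or the player character.
; Touching the player clears CanDisappear, which blocks the timed destruction driven by a Delay on Tick.
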(event `self.ReceiveBeginPlay`
  (`AddComponent|NODE_AddAudioComponent-1`))

(event `self.ReceiveTick`
  (params (DeltaSeconds :type "Float (single-precision)"))
  (`KismetSystemLibrary.Delay` 10.0)
  (if (`self.CanDisappear`)
    (`self.K2_DestroyActor`)))

(event `self.Box.OnComponentBeginOverlap`
  (params (OverlappedComponent :type "PrimitiveComponent Object Reference") (OtherActor :type "Actor Object Reference") (OtherComp :type "PrimitiveComponent Object Reference") (OtherBodyIndex :type Integer) (bFromSweep :type Boolean) (SweepResult :type "HitResult Structure (by ref)"))
  (cast `/Game/Blueprints/Enemies/BP_ParentEnemy` OtherActor
    (:`CastFailed`
      (cast `/Game/Blueprints/Inventory/ItemClasses/BP_ParentItem` OtherActor
        (:`CastFailed`
          (cast `/Game/ThirdPersonBP/Blueprints/ThirdPersonCharacter` OtherActor
            (:`then`
              (set `self.CanDisappear` false))
            (:`CastFailed`
              (`self.K2_DestroyActor`))))))))

(fn `UserConstructionScript`)