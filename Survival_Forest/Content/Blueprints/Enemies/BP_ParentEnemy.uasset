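; Parent enemy Blueprint that handles health, damage and a floating health bar.
; On BeginPlay it adds a widget component holding an EnemyHealthBar linked to itself, which Tick rotates to face the player character.
; AnyDamage subtracts damage reduced by a resistance percent, then either destroys the actor through Death or knocks it back and upward.
; A Damaged flag with a short delay blocks repeat hits during knockback.
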(event `self.ReceiveBeginPlay`
  (bind _returnvalue (`AddComponent|NODE_AddWidgetComponent-0` :`RelativeTransform` (`KismetMathLibrary.MakeTransform` (0.0 0.0 60.0) (struct) (0.5 0.5 0.05))))
  (set `self.Widget` _returnvalue)
  (bind _returnvalue_2 (`|CreateWidget` "/Game/Blueprints/Inventory/Widgets/EnemyHealthBar.EnemyHealthBar_C" null self))
  (`WidgetComponent.SetWidget` _returnvalue _returnvalue_2)
  (`self.K2_AttachToComponent` null "None" "KeepRelative" "KeepRelative" "KeepRelative"))

(event `self.ReceiveTick`
  (params (DeltaSeconds :type "Float (single-precision)"))
  (bind _widget (`self.Widget`))
  (if (`KismetSystemLibrary.IsValid` _widget)
    (`SceneComponent.K2_SetWorldRotation` _widget (`KismetMathLibrary.FindLookAtRotation` (`SceneComponent.K2_GetComponentLocation` _widget) (`self.K2_GetActorLocation` (`GameplayStatics.GetPlayerCharacter` 0))) false false)))

(event `self.ReceiveAnyDamage`
  (params (Damage :type "Float (single-precision)") (DamageType :type "DamageType Object Reference") (InstigatedBy :type "Controller Object Reference") (DamageCauser :type "Actor Object Reference"))
  (bind (_returnvalue_x _returnvalue_y) (`KismetMathLibrary.BreakVector` (* (`self.GetActorForwardVector` self) -10000.0)))
  (if (not (`self.Damaged`))
    (set `self.Damaged` true)
    (bind _output_get (set `self.Health` (- (`self.Health`) (- Damage (* (/ Damage 100.0) (`self.DamageResistancePercent`))))))
    (`KismetSystemLibrary.PrintString` (`KismetStringLibrary.Conv_DoubleToString` _output_get))
    (if (<= (`self.Health`) 0.0)
      (`self.Death`)
      (else
        (`CharacterMovementComponent.AddImpulse` (`self.CharacterMovement`) (`KismetMathLibrary.MakeVector` _returnvalue_x _returnvalue_y 8000.0) false)
        (`KismetSystemLibrary.Delay` 0.8)
        (set `self.Damaged` false)))))

(fn `Death`
  (`self.K2_DestroyActor`))

(fn `UserConstructionScript`)