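; BP_Storage is an item storage container with fixed slots, seeded from StartItems and shown through the player HUD's storage widget.
; AddItem fills free stacks, then empty slots, recursing on overflow and returning any remainder.
; Slot functions remove, swap, merge and move items in from the player inventory, refreshing affected slot widgets.
; Show and Hide toggle the widget and the inventory's StorageOpen flag, with an audio component added on show.
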(event `self.ReceiveBeginPlay`
  (set `self.Slots` (`self.StartItems`))
  (set `self.StorageWidget` (`/Game/Blueprints/HUD/HUD.StorageWidget` (`/Game/Blueprints/Inventory/BP_Inventory.HUDWidget` (`/Game/ThirdPersonBP/Blueprints/ThirdPersonCharacter.InventoryRef` (`self.CharRef`)))))
  (`KismetArrayLibrary.Array_Resize` (`self.Slots`) (`self.AmountOfSlots`)))

(event `UpdateSlotAtIndex`
  (params (index :type Integer))
  (`/Game/Blueprints/Inventory/Widgets/Storage/StorageSlot.UpdateSlot` (`|GetArrayItem` (`/Game/Blueprints/Inventory/Widgets/Storage/StorageWidget.Slotswidgets` (`self.StorageWidget`)) index)))

(fn `AddItem`
  (params (ItemClass :type "/Game/Blueprints/Inventory/ItemClasses/BP_ParentItem Class Reference") (Amount :type Integer))
  (returns (Success :type Boolean) (Rest :type Integer))
  (locals (FoundSlotIndex :type Integer :default 0) (localAmount :type Integer))
  (bind _slots (`self.Slots`))
  (bind _maxstacksize (`self.MaxStackSize`))
  (bind _maxstacksize_2 (`self.MaxStackSize`))
  (bind _foundslotindex (`local.FoundSlotIndex`))
  (if (`.CanBeStacked?_27_37298C0E411C53469A2B8485FA8E1094` (break `/Game/Blueprints/Inventory/Structures/S_ItemInfo` (defaults `/Game/Blueprints/Inventory/BP_Inventory` ItemClass)))
    (bind (_success_ _index) (`self.SearchFreeStack` ItemClass))
    (if _success_
      (set `local.FoundSlotIndex` _index)
      (bind _returnvalue (+ (`.Amount_5_D5C42DA54571DB938AD62A989F1C0456` (break `/Game/Blueprints/Inventory/Structures/S_InventorySlot` (`|GetArrayItem` (`self.Slots`) _index))) Amount))
      (if (> _returnvalue _maxstacksize_2)
        (set `local.localAmount` (- _returnvalue _maxstacksize_2))
        (`KismetArrayLibrary.Array_Set` _slots _foundslotindex (make `/Game/Blueprints/Inventory/Structures/S_InventorySlot` ItemClass (`self.MaxStackSize`)))
        (`self.UpdateSlotAtIndex` (`local.FoundSlotIndex`))
        (bind (_success _rest) (`self.AddItem` ItemClass (`local.localAmount`)))
        (return true _rest)
        (else
          (`KismetArrayLibrary.Array_Set` _slots _foundslotindex (make `/Game/Blueprints/Inventory/Structures/S_InventorySlot` ItemClass _returnvalue))
          (`self.UpdateSlotAtIndex` (`local.FoundSlotIndex`))
          (return true 0)))
      (else
        (bind (_success_2 _index_2) (`self.SearchEmptySlot`))
        (if _success_2
          (bind _output_get (set `local.FoundSlotIndex` _index_2))
          (if (> Amount _maxstacksize)
            (`KismetArrayLibrary.Array_Set` _slots _output_get (make `/Game/Blueprints/Inventory/Structures/S_InventorySlot` ItemClass _maxstacksize))
            (`self.UpdateSlotAtIndex` (`local.FoundSlotIndex`))
            (bind (_success_3 _rest_2) (`self.AddItem` ItemClass (- Amount _maxstacksize)))
            (return true _rest_2)
            (else
              (`KismetArrayLibrary.Array_Set` _slots _output_get (make `/Game/Blueprints/Inventory/Structures/S_InventorySlot` ItemClass Amount))
              (`self.UpdateSlotAtIndex` (`local.FoundSlotIndex`))
              (return true 0)))
          (else
            _))))
    (else
      (bind (_success_4 _index_3) (`self.SearchEmptySlot`))
      (set `local.FoundSlotIndex` _index_3)
      (if _success_4
        (`KismetArrayLibrary.Array_Set` (`self.Slots`) _index_3 (make `/Game/Blueprints/Inventory/Structures/S_InventorySlot` ItemClass 1))
        (`self.UpdateSlotAtIndex` (`local.FoundSlotIndex`))
        (if (> Amount 1)
          (bind (_success_5 _rest_3) (`self.AddItem` ItemClass (- Amount 1)))
          (return true _rest_3)
          (else
            (return true 0)))
        (else
          _))))
  (return false Amount))

(fn `AddItemToIndex`
  (params (index :type Integer) (Amount :type Integer) (item :type "/Game/Blueprints/Inventory/ItemClasses/BP_ParentItem Class Reference"))
  (returns (Success :type Boolean))
  (if (and (`self.IsSlotEmpty?` index) (<= Amount (`self.MaxStackSize`)))
    (`KismetArrayLibrary.Array_Set` (`self.Slots`) index (make `/Game/Blueprints/Inventory/Structures/S_InventorySlot` item Amount))
    (`self.UpdateSlotAtIndex` index)
    (return true)
    (else
      (return false))))

(fn `AddToIndex`
  (params (FromIndex :type Integer) (ToIndex :type Integer))
  (returns (Success :type Boolean))
  (bind _amount (`self.GetAmountAtIndex` FromIndex))
  (bind _amount_2 (`self.GetAmountAtIndex` ToIndex))
  (bind _slots (`self.Slots`))
  (bind _maxstacksize (`self.MaxStackSize`))
  (bind (_output_itemclass _output_amount) (break `/Game/Blueprints/Inventory/Structures/S_InventorySlot` (`|GetArrayItem` (`self.Slots`) ToIndex)))
  (bind _output_itemclass_2 (break `/Game/Blueprints/Inventory/Structures/S_InventorySlot` (`|GetArrayItem` (`self.Slots`) FromIndex)))
  (if (and (== _output_itemclass_2 _output_itemclass) (< _output_amount (`self.MaxStackSize`)) (`.CanBeStacked?_27_37298C0E411C53469A2B8485FA8E1094` (break `/Game/Blueprints/Inventory/Structures/S_ItemInfo` (`.ItemInfo` (`self.GetInfoAboutSlot` FromIndex)))))
    (if (>= (- (`self.MaxStackSize`) _amount_2) _amount)
      (`KismetArrayLibrary.Array_Set` _slots ToIndex (make `/Game/Blueprints/Inventory/Structures/S_InventorySlot` _output_itemclass_2 (+ _amount_2 _amount)))
      (`KismetArrayLibrary.Array_Set` _slots FromIndex (make `/Game/Blueprints/Inventory/Structures/S_InventorySlot` null))
      (else
        (`KismetArrayLibrary.Array_Set` _slots FromIndex (make `/Game/Blueprints/Inventory/Structures/S_InventorySlot` _output_itemclass_2 (- (`self.GetAmountAtIndex` FromIndex) (- _maxstacksize (`self.GetAmountAtIndex` ToIndex)))))
        (`KismetArrayLibrary.Array_Set` _slots ToIndex (make `/Game/Blueprints/Inventory/Structures/S_InventorySlot` _output_itemclass_2 _maxstacksize))))
    (`self.UpdateSlotAtIndex` FromIndex)
    (`self.UpdateSlotAtIndex` ToIndex)
    (return true)
    (else
      (return false))))

(fn `GetAmountAtIndex`
  (params (Index :type Integer))
  (returns (Amount :type Integer))
  (return (`.Amount_5_D5C42DA54571DB938AD62A989F1C0456` (break `/Game/Blueprints/Inventory/Structures/S_InventorySlot` (`|GetArrayItem` (`self.Slots`) Index)))))

(fn `GetInfoAboutSlot`
  (params (Index :type Integer))
  (returns (`IsSlotEmpty?` :type Boolean) (ItemInfo :type "/Game/Blueprints/Inventory/Structures/S_ItemInfo Structure") (Amount :type Integer))
  (bind (_itemclass _amount) (break `/Game/Blueprints/Inventory/Structures/S_InventorySlot` (`|GetArrayItem` (`self.Slots`) Index)))
  (if (`KismetSystemLibrary.IsValidClass` _itemclass)
    (return false (defaults `/Game/Blueprints/Inventory/BP_Inventory` _itemclass) _amount)
    (else
      (return true (struct) 0))))

(fn `HideStorage`
  (`Widget.SetVisibility` (`self.StorageWidget`) "Hidden")
  (set `/Game/Blueprints/Inventory/BP_Inventory.StorageOpen?` false (`/Game/ThirdPersonBP/Blueprints/ThirdPersonCharacter.InventoryRef` (`self.CharRef`)))
  (return))

(fn `IncreaseAmountAtIndex`
  (params (index :type Integer) (Amount :type Integer))
  (returns (Success :type Boolean))
  (bind _slots (`self.Slots`))
  (bind (_output_itemclass _output_amount) (break `/Game/Blueprints/Inventory/Structures/S_InventorySlot` (`|GetArrayItem` _slots)))
  (if (and (not (`self.IsSlotEmpty?` index)) (<= (+ (`self.GetAmountAtIndex` index) Amount) (`self.MaxStackSize`)))
    (`KismetArrayLibrary.Array_Set` _slots index (make `/Game/Blueprints/Inventory/Structures/S_InventorySlot` _output_itemclass (+ _output_amount Amount)))
    (`self.UpdateSlotAtIndex` index)
    (return true)
    (else
      (return false))))

(fn `IsSlotEmpty?`
  (params (Index :type Integer))
  (returns (`Empty?` :type Boolean))
  (return (not (`KismetSystemLibrary.IsValidClass` (`.ItemClass_2_117ED78645722B73FB101F9F6C3FC4DF` (break `/Game/Blueprints/Inventory/Structures/S_InventorySlot` (`|GetArrayItem` (`self.Slots`) Index)))))))

(fn `MoveFromInventoryToStorage`
  (params (inventory :type "/Game/Blueprints/Inventory/BP_Inventory Object Reference") (InventoryIndex :type Integer) (StorageIndex :type Integer))
  (returns (Success :type Boolean))
  (locals (AmountToAdd :type Integer))
  (bind _amount (`/Game/Blueprints/Inventory/BP_Inventory.GetAmountAtIndex` inventory InventoryIndex))
  (bind _returnvalue (- (`self.MaxStackSize`) (`self.GetAmountAtIndex` StorageIndex)))
  (bind _output_itemclass (break `/Game/Blueprints/Inventory/Structures/S_InventorySlot` (`|GetArrayItem` (`/Game/Blueprints/Inventory/BP_Inventory.Slots` inventory) InventoryIndex)))
  (bind _output_itemclass_2 (break `/Game/Blueprints/Inventory/Structures/S_InventorySlot` (`|GetArrayItem` (`self.Slots`) StorageIndex)))
  (bind (_output_itemclass_3 _output_amount) (break `/Game/Blueprints/Inventory/Structures/S_InventorySlot` (`|GetArrayItem` (`/Game/Blueprints/Inventory/BP_Inventory.Slots` inventory) InventoryIndex)))
  (if (`self.IsSlotEmpty?` StorageIndex)
    (bind _output_get (set `local.AmountToAdd` (`/Game/Blueprints/Inventory/BP_Inventory.GetAmountAtIndex` inventory InventoryIndex)))
    (bind _success (`self.AddItemToIndex` StorageIndex _output_get _output_itemclass))
    (if _success
      (`/Game/Blueprints/Inventory/BP_Inventory.RemoveItemAtIndex` inventory InventoryIndex _output_get)
      (return true)
      (else
        _))
    (elif (and (== _output_itemclass_2 _output_itemclass_3) (`.CanBeStacked?_27_37298C0E411C53469A2B8485FA8E1094` (break `/Game/Blueprints/Inventory/Structures/S_ItemInfo` (`.ItemInfo` (`self.GetInfoAboutSlot` StorageIndex)))) (<= (+ (`self.GetAmountAtIndex` StorageIndex) _output_amount) (`self.MaxStackSize`)))
      (bind _output_get_2 (set `local.AmountToAdd` (`KismetMathLibrary.SelectInt` _returnvalue _amount (> _amount _returnvalue))))
      (bind _success_2 (`self.IncreaseAmountAtIndex` StorageIndex _output_get_2))
      (if _success_2
        (`/Game/Blueprints/Inventory/BP_Inventory.RemoveItemAtIndex` inventory InventoryIndex (`local.AmountToAdd`))
        (return true)
        (else
          _))))
  (return false))

(fn `RemoveItemAtIndex`
  (params (index :type Integer) (Amount :type Integer))
  (returns (Success :type Boolean))
  (locals (localindex :type Boolean) (localamount :type Boolean))
  (bind _slots (`self.Slots`))
  (bind (_output_itemclass _output_amount) (break `/Game/Blueprints/Inventory/Structures/S_InventorySlot` (`|GetArrayItem` _slots index)))
  (if (and (not (`self.IsSlotEmpty?` index)) (> Amount 0))
    (if (>= Amount (`self.GetAmountAtIndex` index))
      (`KismetArrayLibrary.Array_Set` (`self.Slots`) index (make `/Game/Blueprints/Inventory/Structures/S_InventorySlot` null))
      (`self.UpdateSlotAtIndex` index)
      (return true)
      (else
        (`KismetArrayLibrary.Array_Set` _slots index (make `/Game/Blueprints/Inventory/Structures/S_InventorySlot` _output_itemclass (- _output_amount Amount)))
        (`self.UpdateSlotAtIndex` index)
        (return true)))
    (else
      (return false))))

(fn `SearchEmptySlot`
  (returns (Success :type Boolean) (index :type Integer))
  (locals (localbool :type Boolean) (localindex :type Integer))
  (for (_array_element _array_index) (`self.Slots`)
    (if (not (`KismetSystemLibrary.IsValidClass` (`.ItemClass_2_117ED78645722B73FB101F9F6C3FC4DF` (break `/Game/Blueprints/Inventory/Structures/S_InventorySlot` _array_element))))
      (set `local.localbool` true)
      (set `local.localindex` _array_index)
      (break)))
  (return (`local.localbool`) (`local.localindex`)))

(fn `SearchFreeStack`
  (params (ItemClass :type "/Game/Blueprints/Inventory/ItemClasses/BP_ParentItem Class Reference"))
  (returns (`Success?` :type Boolean) (Index :type Integer))
  (locals (localbool :type Boolean :default false) (localindex :type Integer))
  (for (_array_element _array_index) (`self.Slots`)
    (bind (_itemclass _amount) (break `/Game/Blueprints/Inventory/Structures/S_InventorySlot` _array_element))
    (if (`KismetSystemLibrary.IsValidClass` _itemclass)
      (if (and (== _itemclass ItemClass) (< _amount (`self.MaxStackSize`)))
        (set `local.localindex` _array_index)
        (set `local.localbool` true)
        (break))))
  (return (`local.localbool`) (`local.localindex`)))

(fn `ShowStorage`
  (`Widget.SetVisibility` (`self.StorageWidget`) "Visible")
  (set `/Game/Blueprints/Inventory/BP_Inventory.StorageOpen?` true (`/Game/ThirdPersonBP/Blueprints/ThirdPersonCharacter.InventoryRef` (`self.CharRef`)))
  (`AddComponent|NODE_AddAudioComponent-0`)
  (return))

(fn `SwapSlots`
  (params (index1 :type Integer) (index2 :type Integer))
  (returns (Success :type Boolean))
  (locals (LocalSlot2 :type "/Game/Blueprints/Inventory/Structures/S_InventorySlot Structure"))
  (bind _slots (`self.Slots`))
  (bind _returnvalue (`KismetArrayLibrary.Array_LastIndex` (`self.Slots`)))
  (if (or (> index1 _returnvalue) (> index2 _returnvalue))
    (return false)
    (else
      (set `local.LocalSlot2` (`|GetArrayItem` (`self.Slots`) index2))
      (`KismetArrayLibrary.Array_Set` _slots index2 (`|GetArrayItem` _slots index1))
      (`KismetArrayLibrary.Array_Set` _slots index1 (`local.LocalSlot2`))
      (`self.UpdateSlotAtIndex` index1)
      (`self.UpdateSlotAtIndex` index2)
      (return true))))

(fn `UserConstructionScript`)