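; Player inventory that stores items as class-and-amount slots, with stacking, splitting, merging, swapping, removal and transfers from storage.
; AddItem fills free stacks or empty slots, recursing on overflow and returning what did not fit.
; Slot changes refresh the inventory widget and bound hotkeys, and most also refresh the crafting menu.
; Using an item, directly or by hotkey, raises Health, Hunger or Thirst for consumables and spawns the item actor to call Used.
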(event `self.ReceiveBeginPlay`
  (`KismetArrayLibrary.Array_Resize` (`self.Slots`) (`self.AmountOfSlots`))
  (set `self.Showhotkeys?` (`/Game/ThirdPersonBP/Blueprints/ThirdPersonCharacter.ShowHotkeys?` (`self.CharRef`))))

(event `UpdateSlotAtIndex`
  (params (index :type Integer))
  (`/Game/Blueprints/Inventory/Widgets/InventorySlot.UpdateSlot` (`|GetArrayItem` (`/Game/Blueprints/Inventory/Widgets/Inventorywidget.Slotswidgets` (`self.InventoryWidget`)) index))
  (`self.UpdateHotkeyForIndex` index))

(event `UseItemAtindex`
  (params (index :type Integer))
  (bind (_isslotempty_ _iteminfo) (`self.GetInfoAboutSlot` index))
  (bind _charref (`self.CharRef`))
  (bind _output_itemclass (break `/Game/Blueprints/Inventory/Structures/S_InventorySlot` (`|GetArrayItem` (`self.Slots`) index)))
  (bind _returnvalue (+ (`/Game/ThirdPersonBP/Blueprints/ThirdPersonCharacter.Thirst` _charref) (`.ItemImportantParametr_41_63C1C7C3430F243A349D449146DBA7DF` (break `/Game/Blueprints/Inventory/Structures/S_ItemInfo` _iteminfo))))
  (bind _returnvalue_2 (+ (`/Game/ThirdPersonBP/Blueprints/ThirdPersonCharacter.Health` _charref) (`.ItemImportantParametr_41_63C1C7C3430F243A349D449146DBA7DF` (break `/Game/Blueprints/Inventory/Structures/S_ItemInfo` _iteminfo))))
  (bind _returnvalue_3 (+ (`/Game/ThirdPersonBP/Blueprints/ThirdPersonCharacter.Hunger` _charref) (`.ItemImportantParametr_41_63C1C7C3430F243A349D449146DBA7DF` (break `/Game/Blueprints/Inventory/Structures/S_ItemInfo` _iteminfo))))
  (if (select `/Game/Blueprints/Inventory/Enums/E_ItemCategories` (`.Category_28_FBF63B474F26E3585A561E8E2AAC38B3` (break `/Game/Blueprints/Inventory/Structures/S_ItemInfo` _iteminfo)) :`NewEnumerator0` true)
    (`|MultiGate` false false (select `/Game/Blueprints/Inventory/Enums/E_ItemSubCategories` (`.SubCategory_38_3D035FDA4D0CDA30F93EF1840A9BF988` (break `/Game/Blueprints/Inventory/Structures/S_ItemInfo` _iteminfo)) :`NewEnumerator1` 1 :`NewEnumerator2` 2 :`NewEnumerator4` 3) :!label _label
      (:`Out 0`
        (if (< _returnvalue_2 1.0)
          (set `/Game/ThirdPersonBP/Blueprints/ThirdPersonCharacter.Health` _returnvalue_2 _charref)
          (else
            (set `/Game/ThirdPersonBP/Blueprints/ThirdPersonCharacter.Health` 1.0 _charref))))
      (:`Out 1`
        (if (< _returnvalue_3 1.0)
          (set `/Game/ThirdPersonBP/Blueprints/ThirdPersonCharacter.Hunger` _returnvalue_3 _charref)
          (else
            (set `/Game/ThirdPersonBP/Blueprints/ThirdPersonCharacter.Hunger` 1.0 _charref))))
      (:`Out 2`
        (if (< _returnvalue 1.0)
          (set `/Game/ThirdPersonBP/Blueprints/ThirdPersonCharacter.Thirst` _returnvalue _charref)
          (else
            (set `/Game/ThirdPersonBP/Blueprints/ThirdPersonCharacter.Thirst` 1.0 _charref))))))
  (if (`KismetSystemLibrary.IsValidClass` _output_itemclass)
    (bind _returnvalue_4 (`|SpawnActorFromClass` _output_itemclass (`KismetMathLibrary.MakeTransform` (0.0 0.0 0.0)) "AlwaysSpawn" "OverrideRootScale" null self index null))
    (`/Game/Blueprints/Inventory/ItemClasses/BP_ParentItem.Used` _returnvalue_4)
    (goto _label :!via `Reset`)))

(fn `AddItem`
  (params (ItemClass :type "/Game/Blueprints/Inventory/ItemClasses/BP_ParentItem Class Reference") (Amount :type Integer))
  (returns (Success :type Boolean) (Rest :type Integer))
  (locals (FoundSlotIndex :type Integer :default 0) (localAmount :type Integer))
  (bind _slots (`self.Slots`))
  (bind _maxstacksize (`self.MaxStackSize`))
  (bind _maxstacksize_2 (`self.MaxStackSize`))
  (bind _foundslotindex (`local.FoundSlotIndex`))
  (if (`.CanBeStacked?_27_37298C0E411C53469A2B8485FA8E1094` (break `/Game/Blueprints/Inventory/Structures/S_ItemInfo` (defaults `/Game/Blueprints/Inventory/BP_Inventory` ItemClass)))
    (bind (_success_ _index) (`self.SearchFreeStack` ItemClass))
    (if _success_
      (set `local.FoundSlotIndex` _index)
      (bind _returnvalue (+ (`.Amount_5_D5C42DA54571DB938AD62A989F1C0456` (break `/Game/Blueprints/Inventory/Structures/S_InventorySlot` (`|GetArrayItem` (`self.Slots`) _index))) Amount))
      (if (> _returnvalue _maxstacksize_2)
        (set `local.localAmount` (- _returnvalue _maxstacksize_2))
        (`KismetArrayLibrary.Array_Set` _slots _foundslotindex (make `/Game/Blueprints/Inventory/Structures/S_InventorySlot` ItemClass (`self.MaxStackSize`)))
        (`self.UpdateSlotAtIndex` (`local.FoundSlotIndex`))
        (bind (_success _rest) (`self.AddItem` ItemClass (`local.localAmount`)))
        (`self.UpdateCraftingMenu`)
        (return true _rest)
        (else
          (`KismetArrayLibrary.Array_Set` _slots _foundslotindex (make `/Game/Blueprints/Inventory/Structures/S_InventorySlot` ItemClass _returnvalue))
          (`self.UpdateSlotAtIndex` (`local.FoundSlotIndex`))
          (return true 0)))
      (else
        (bind (_success_2 _index_2) (`self.SearchEmptySlot`))
        (if _success_2
          (bind _output_get (set `local.FoundSlotIndex` _index_2))
          (if (> Amount _maxstacksize)
            (`KismetArrayLibrary.Array_Set` _slots _output_get (make `/Game/Blueprints/Inventory/Structures/S_InventorySlot` ItemClass _maxstacksize))
            (`self.UpdateSlotAtIndex` (`local.FoundSlotIndex`))
            (bind (_success_3 _rest_2) (`self.AddItem` ItemClass (- Amount _maxstacksize)))
            (`self.UpdateCraftingMenu`)
            (return true _rest_2)
            (else
              (`KismetArrayLibrary.Array_Set` _slots _output_get (make `/Game/Blueprints/Inventory/Structures/S_InventorySlot` ItemClass Amount))
              (`self.UpdateSlotAtIndex` (`local.FoundSlotIndex`))
              (`self.UpdateCraftingMenu`)
              (return true 0)))
          (else
            _))))
    (else
      (bind (_success_4 _index_3) (`self.SearchEmptySlot`))
      (set `local.FoundSlotIndex` _index_3)
      (if _success_4
        (`KismetArrayLibrary.Array_Set` (`self.Slots`) _index_3 (make `/Game/Blueprints/Inventory/Structures/S_InventorySlot` ItemClass 1))
        (`self.UpdateSlotAtIndex` (`local.FoundSlotIndex`))
        (if (> Amount 1)
          (bind (_success_5 _rest_3) (`self.AddItem` ItemClass (- Amount 1)))
          (`self.UpdateCraftingMenu`)
          (return true _rest_3)
          (else
            (`self.UpdateCraftingMenu`)
            (return true 0)))
        (else
          _))))
  (return false Amount))

(fn `AddItemToIndex`
  (params (index :type Integer) (Amount :type Integer) (item :type "/Game/Blueprints/Inventory/ItemClasses/BP_ParentItem Class Reference"))
  (returns (Success :type Boolean))
  (if (and (`self.IsSlotEmpty?` index) (<= Amount (`self.MaxStackSize`)))
    (`KismetArrayLibrary.Array_Set` (`self.Slots`) index (make `/Game/Blueprints/Inventory/Structures/S_InventorySlot` item Amount))
    (`self.UpdateSlotAtIndex` index)
    (`self.UpdateCraftingMenu`)
    (return true)
    (else
      (return false))))

(fn `AddToIndex`
  (params (FromIndex :type Integer) (ToIndex :type Integer))
  (returns (Success :type Boolean))
  (bind _amount (`self.GetAmountAtIndex` FromIndex))
  (bind _amount_2 (`self.GetAmountAtIndex` ToIndex))
  (bind _slots (`self.Slots`))
  (bind _maxstacksize (`self.MaxStackSize`))
  (bind (_output_itemclass _output_amount) (break `/Game/Blueprints/Inventory/Structures/S_InventorySlot` (`|GetArrayItem` (`self.Slots`) ToIndex)))
  (bind _output_itemclass_2 (break `/Game/Blueprints/Inventory/Structures/S_InventorySlot` (`|GetArrayItem` (`self.Slots`) FromIndex)))
  (if (and (== _output_itemclass_2 _output_itemclass) (< _output_amount (`self.MaxStackSize`)) (`.CanBeStacked?_27_37298C0E411C53469A2B8485FA8E1094` (break `/Game/Blueprints/Inventory/Structures/S_ItemInfo` (`.ItemInfo` (`self.GetInfoAboutSlot` FromIndex)))))
    (if (>= (- (`self.MaxStackSize`) _amount_2) _amount)
      (`KismetArrayLibrary.Array_Set` _slots ToIndex (make `/Game/Blueprints/Inventory/Structures/S_InventorySlot` _output_itemclass_2 (+ _amount_2 _amount)))
      (`KismetArrayLibrary.Array_Set` _slots FromIndex (make `/Game/Blueprints/Inventory/Structures/S_InventorySlot` null))
      (else
        (`KismetArrayLibrary.Array_Set` _slots FromIndex (make `/Game/Blueprints/Inventory/Structures/S_InventorySlot` _output_itemclass_2 (- (`self.GetAmountAtIndex` FromIndex) (- _maxstacksize (`self.GetAmountAtIndex` ToIndex)))))
        (`KismetArrayLibrary.Array_Set` _slots ToIndex (make `/Game/Blueprints/Inventory/Structures/S_InventorySlot` _output_itemclass_2 _maxstacksize))))
    (`self.UpdateSlotAtIndex` FromIndex)
    (`self.UpdateSlotAtIndex` ToIndex)
    (return true)
    (else
      (return false))))

(fn `GetAmountAtIndex`
  (params (Index :type Integer))
  (returns (Amount :type Integer))
  (return (`.Amount_5_D5C42DA54571DB938AD62A989F1C0456` (break `/Game/Blueprints/Inventory/Structures/S_InventorySlot` (`|GetArrayItem` (`self.Slots`) Index)))))

(fn `GetInfoAboutSlot`
  (params (Index :type Integer))
  (returns (`IsSlotEmpty?` :type Boolean) (ItemInfo :type "/Game/Blueprints/Inventory/Structures/S_ItemInfo Structure") (Amount :type Integer))
  (bind (_itemclass _amount) (break `/Game/Blueprints/Inventory/Structures/S_InventorySlot` (`|GetArrayItem` (`self.Slots`) Index)))
  (if (`KismetSystemLibrary.IsValidClass` _itemclass)
    (return false (defaults `/Game/Blueprints/Inventory/BP_Inventory` _itemclass) _amount)
    (else
      (return true (struct) 0))))

(fn `GetTotalAmountOfItem`
  (params (item :type "/Game/Blueprints/Inventory/ItemClasses/BP_ParentItem Class Reference"))
  (returns (TotalAmount :type Integer) (SlotIndices :type "Array of Integer"))
  (locals (LocalAmount :type Integer) (LocalSlotIndices :type "Array of Integer"))
  (for (_array_element _array_index) (`self.Slots`)
    (if (`KismetSystemLibrary.IsValidClass` (break `/Game/Blueprints/Inventory/Structures/S_InventorySlot` _array_element))
      (if (== (break `/Game/Blueprints/Inventory/Structures/S_InventorySlot` _array_element) item)
        (`KismetArrayLibrary.Array_Add` (`local.LocalSlotIndices`) _array_index)
        (set `local.LocalAmount` (+ (`local.LocalAmount`) (`.Amount_5_D5C42DA54571DB938AD62A989F1C0456` (break `/Game/Blueprints/Inventory/Structures/S_InventorySlot` _array_element)))))))
  (return (`local.LocalAmount`) (`local.LocalSlotIndices`)))

(fn `HandleHotkeyPress`
  (params (PressedKey :type "Key Structure" :default "None"))
  (if (`self.Showhotkeys?`)
    (for _array_element (`/Game/Blueprints/HUD/HUD.HotkeyWidgets` (`self.HUDWidget`))
      (bind _hotkeyslot (`/Game/Blueprints/HUD/Hotkey.HotkeySlot` _array_element))
      (if (and (== (`/Game/Blueprints/HUD/Hotkey.Key` _array_element) PressedKey) (not (`/Game/Blueprints/HUD/HotkeySlot.Empty?` _hotkeyslot)))
        (`self.UseItemAtindex` (`/Game/Blueprints/HUD/HotkeySlot.InventoryIndex` _hotkeyslot))
        (break))))
  (return))

(fn `HandleSwapForHotkeys`
  (params (index1 :type Integer) (index2 :type Integer))
  (if (`self.Showhotkeys?`)
    (for _array_element (`/Game/Blueprints/HUD/HUD.HotkeyWidgets` (`self.HUDWidget`))
      (bind _hotkeyslot (`/Game/Blueprints/HUD/Hotkey.HotkeySlot` _array_element))
      (if (not (`/Game/Blueprints/HUD/HotkeySlot.Empty?` _hotkeyslot))
        (bind _inventoryindex (`/Game/Blueprints/HUD/HotkeySlot.InventoryIndex` _hotkeyslot))
        (if (== _inventoryindex index1)
          (set `/Game/Blueprints/HUD/HotkeySlot.InventoryIndex` index2 _hotkeyslot)
          (elif (== _inventoryindex index2)
            (set `/Game/Blueprints/HUD/HotkeySlot.InventoryIndex` index1 _hotkeyslot))))))
  (return))

(fn `HideInventory`
  (params (`CloseStorage?` :type Boolean))
  (bind _inventorywidget (`self.InventoryWidget`))
  (if (and `CloseStorage?` (`self.StorageOpen?`))
    (`/Game/Blueprints/Inventory/ItemClasses/BP_Chest.OnStorageClosed` (`/Game/Blueprints/Inventory/BP_Storage.Chest` (`/Game/Blueprints/Inventory/Widgets/Storage/StorageWidget.StorageRef` (`/Game/Blueprints/HUD/HUD.StorageWidget` (`self.HUDWidget`))))))
  (`Widget.SetVisibility` _inventorywidget "Hidden")
  (set `self.InventoryOpen?` false)
  (`Widget.SetIsEnabled` _inventorywidget false)
  (return))

(fn `IncreaseAmountAtIndex`
  (params (index :type Integer) (Amount :type Integer))
  (returns (Success :type Boolean))
  (bind _slots (`self.Slots`))
  (bind (_output_itemclass _output_amount) (break `/Game/Blueprints/Inventory/Structures/S_InventorySlot` (`|GetArrayItem` _slots)))
  (if (and (not (`self.IsSlotEmpty?` index)) (<= (+ (`self.GetAmountAtIndex` index) Amount) (`self.MaxStackSize`)))
    (`KismetArrayLibrary.Array_Set` _slots index (make `/Game/Blueprints/Inventory/Structures/S_InventorySlot` _output_itemclass (+ _output_amount Amount)))
    (`self.UpdateSlotAtIndex` index)
    (`self.UpdateCraftingMenu`)
    (return true)
    (else
      (return false))))

(fn `IsSlotEmpty?`
  (params (Index :type Integer))
  (returns (`Empty?` :type Boolean))
  (return (not (`KismetSystemLibrary.IsValidClass` (`.ItemClass_2_117ED78645722B73FB101F9F6C3FC4DF` (break `/Game/Blueprints/Inventory/Structures/S_InventorySlot` (`|GetArrayItem` (`self.Slots`) Index)))))))

(fn `MoveFromStorageToInventory`
  (params (Storage :type "/Game/Blueprints/Inventory/BP_Storage Object Reference") (StorageIndex :type Integer) (InventoryIndex :type Integer))
  (returns (Success :type Boolean))
  (locals (AmountToAdd :type Integer))
  (bind _amount (`/Game/Blueprints/Inventory/BP_Storage.GetAmountAtIndex` Storage StorageIndex))
  (bind _returnvalue (- (`self.MaxStackSize`) (`self.GetAmountAtIndex` InventoryIndex)))
  (bind _output_itemclass (break `/Game/Blueprints/Inventory/Structures/S_InventorySlot` (`|GetArrayItem` (`/Game/Blueprints/Inventory/BP_Storage.Slots` Storage) StorageIndex)))
  (bind _output_itemclass_2 (break `/Game/Blueprints/Inventory/Structures/S_InventorySlot` (`|GetArrayItem` (`self.Slots`) InventoryIndex)))
  (bind (_output_itemclass_3 _output_amount) (break `/Game/Blueprints/Inventory/Structures/S_InventorySlot` (`|GetArrayItem` (`/Game/Blueprints/Inventory/BP_Storage.Slots` Storage) StorageIndex)))
  (if (`self.IsSlotEmpty?` InventoryIndex)
    (bind _output_get (set `local.AmountToAdd` (`/Game/Blueprints/Inventory/BP_Storage.GetAmountAtIndex` Storage StorageIndex)))
    (bind _success (`self.AddItemToIndex` InventoryIndex _output_get _output_itemclass))
    (if _success
      (`/Game/Blueprints/Inventory/BP_Storage.RemoveItemAtIndex` Storage StorageIndex _output_get)
      (return true)
      (else
        _))
    (elif (and (== _output_itemclass_2 _output_itemclass_3) (`.CanBeStacked?_27_37298C0E411C53469A2B8485FA8E1094` (break `/Game/Blueprints/Inventory/Structures/S_ItemInfo` (`.ItemInfo` (`self.GetInfoAboutSlot` InventoryIndex)))) (<= (+ (`self.GetAmountAtIndex` InventoryIndex) _output_amount) (`self.MaxStackSize`)))
      (bind _output_get_2 (set `local.AmountToAdd` (`KismetMathLibrary.SelectInt` _returnvalue _amount (> _amount _returnvalue))))
      (bind _success_2 (`self.IncreaseAmountAtIndex` InventoryIndex _output_get_2))
      (if _success_2
        (`/Game/Blueprints/Inventory/BP_Storage.RemoveItemAtIndex` Storage StorageIndex (`local.AmountToAdd`))
        (return true)
        (else
          _))))
  (return false))

(fn `RemoveItem`
  (params (Item :type "/Game/Blueprints/Inventory/ItemClasses/BP_ParentItem Class Reference") (Amount :type Integer))
  (returns (Success :type Boolean))
  (locals (AmountToRemove :type Integer))
  (bind (_totalamount _slotindices) (`self.GetTotalAmountOfItem` Item))
  (if (>= _totalamount Amount)
    (set `local.AmountToRemove` Amount)
    (for _array_element _slotindices
      (bind _amount (`self.GetAmountAtIndex` _array_element))
      (if (< _amount (`local.AmountToRemove`))
        (set `local.AmountToRemove` (- (`local.AmountToRemove`) _amount))
        (`self.RemoveItemAtIndex` _array_element _amount)
        (else
          (`self.RemoveItemAtIndex` _array_element (`local.AmountToRemove`))
          (set `local.AmountToRemove` 0)
          (break))))
    (return true)
    (else
      (return false))))

(fn `RemoveItemAtIndex`
  (params (index :type Integer) (Amount :type Integer))
  (returns (Success :type Boolean))
  (locals (localindex :type Boolean) (localamount :type Boolean))
  (bind _slots (`self.Slots`))
  (bind (_output_itemclass _output_amount) (break `/Game/Blueprints/Inventory/Structures/S_InventorySlot` (`|GetArrayItem` _slots index)))
  (if (and (not (`self.IsSlotEmpty?` index)) (> Amount 0))
    (if (>= Amount (`self.GetAmountAtIndex` index))
      (`KismetArrayLibrary.Array_Set` (`self.Slots`) index (make `/Game/Blueprints/Inventory/Structures/S_InventorySlot` null))
      (`self.UpdateSlotAtIndex` index)
      (`self.UpdateCraftingMenu`)
      (return true)
      (else
        (`KismetArrayLibrary.Array_Set` _slots index (make `/Game/Blueprints/Inventory/Structures/S_InventorySlot` _output_itemclass (- _output_amount Amount)))
        (`self.UpdateSlotAtIndex` index)
        (`self.UpdateCraftingMenu`)
        (return true)))
    (else
      (return false))))

(fn `SearchEmptySlot`
  (returns (Success :type Boolean) (index :type Integer))
  (locals (localbool :type Boolean) (localindex :type Integer))
  (for (_array_element _array_index) (`self.Slots`)
    (if (not (`KismetSystemLibrary.IsValidClass` (`.ItemClass_2_117ED78645722B73FB101F9F6C3FC4DF` (break `/Game/Blueprints/Inventory/Structures/S_InventorySlot` _array_element))))
      (set `local.localbool` true)
      (set `local.localindex` _array_index)
      (break)))
  (return (`local.localbool`) (`local.localindex`)))

(fn `SearchFreeStack`
  (params (ItemClass :type "/Game/Blueprints/Inventory/ItemClasses/BP_ParentItem Class Reference"))
  (returns (`Success?` :type Boolean) (Index :type Integer))
  (locals (localbool :type Boolean :default false) (localindex :type Integer))
  (for (_array_element _array_index) (`self.Slots`)
    (bind (_itemclass _amount) (break `/Game/Blueprints/Inventory/Structures/S_InventorySlot` _array_element))
    (if (`KismetSystemLibrary.IsValidClass` _itemclass)
      (if (and (== _itemclass ItemClass) (< _amount (`self.MaxStackSize`)))
        (set `local.localindex` _array_index)
        (set `local.localbool` true)
        (break))))
  (return (`local.localbool`) (`local.localindex`)))

(fn `ShowInventory`
  (bind _inventorywidget (`self.InventoryWidget`))
  (`Widget.SetVisibility` _inventorywidget "Visible")
  (set `self.InventoryOpen?` true)
  (`Widget.SetIsEnabled` _inventorywidget true)
  (return))

(fn `SplitStack`
  (params (StackIndex :type Integer) (Amount :type Integer))
  (returns (Success :type Boolean))
  (bind (_isslotempty_ _iteminfo _amount) (`self.GetInfoAboutSlot` StackIndex))
  (bind _slots (`self.Slots`))
  (bind (_output_itemclass _output_amount) (break `/Game/Blueprints/Inventory/Structures/S_InventorySlot` (`|GetArrayItem` _slots StackIndex)))
  (if (`self.IsSlotEmpty?` StackIndex)
    (return false)
    (else
      (if (and (`.CanBeStacked?_27_37298C0E411C53469A2B8485FA8E1094` (break `/Game/Blueprints/Inventory/Structures/S_ItemInfo` _iteminfo)) (> _amount Amount))
        (bind (_success _index) (`self.SearchEmptySlot`))
        (if _success
          (`KismetArrayLibrary.Array_Set` _slots StackIndex (make `/Game/Blueprints/Inventory/Structures/S_InventorySlot` _output_itemclass (- _output_amount Amount)))
          (`KismetArrayLibrary.Array_Set` _slots _index (make `/Game/Blueprints/Inventory/Structures/S_InventorySlot` _output_itemclass Amount))
          (`self.UpdateSlotAtIndex` StackIndex)
          (`self.UpdateSlotAtIndex` _index)
          (return true)
          (else
            _)))
      (return false))))

(fn `SplitStackToIndex`
  (params (FromIndex :type Integer) (ToIndex :type Integer) (AmountToSplit :type Integer))
  (returns (Success :type Boolean))
  (bind (_isslotempty_ _iteminfo _amount) (`self.GetInfoAboutSlot` 0))
  (bind _slots (`self.Slots`))
  (bind (_output_itemclass _output_amount) (break `/Game/Blueprints/Inventory/Structures/S_InventorySlot` (`|GetArrayItem` _slots FromIndex)))
  (if (and (not (`self.IsSlotEmpty?` FromIndex)) (`self.IsSlotEmpty?` ToIndex) (`.CanBeStacked?_27_37298C0E411C53469A2B8485FA8E1094` (break `/Game/Blueprints/Inventory/Structures/S_ItemInfo` _iteminfo)) (> _amount 1) (> _amount AmountToSplit))
    (`KismetArrayLibrary.Array_Set` _slots FromIndex (make `/Game/Blueprints/Inventory/Structures/S_InventorySlot` _output_itemclass (- _output_amount AmountToSplit)))
    (`KismetArrayLibrary.Array_Set` _slots ToIndex (make `/Game/Blueprints/Inventory/Structures/S_InventorySlot` _output_itemclass AmountToSplit))
    (`self.UpdateSlotAtIndex` FromIndex)
    (`self.UpdateSlotAtIndex` ToIndex)
    (return true)
    (else
      (return false))))

(fn `SwapSlots`
  (params (index1 :type Integer) (index2 :type Integer))
  (returns (Success :type Boolean))
  (locals (LocalSlot2 :type "/Game/Blueprints/Inventory/Structures/S_InventorySlot Structure"))
  (bind _slots (`self.Slots`))
  (bind _returnvalue (`KismetArrayLibrary.Array_LastIndex` (`self.Slots`)))
  (if (or (> index1 _returnvalue) (> index2 _returnvalue))
    (return false)
    (else
      (set `local.LocalSlot2` (`|GetArrayItem` (`self.Slots`) index2))
      (`self.HandleSwapForHotkeys` index1 index2)
      (`KismetArrayLibrary.Array_Set` _slots index2 (`|GetArrayItem` _slots index1))
      (`KismetArrayLibrary.Array_Set` _slots index1 (`local.LocalSlot2`))
      (`self.UpdateSlotAtIndex` index1)
      (`self.UpdateSlotAtIndex` index2)
      (`self.UpdateCraftingMenu`)
      (return true))))

(fn `UpdateCraftingMenu`
  (bind _craftmenu (`/Game/Blueprints/HUD/HUD.CraftMenu` (`self.HUDWidget`)))
  (bind _currentitemclass (`/Game/Blueprints/Inventory/Widgets/CraftMenu.CurrentItemClass` _craftmenu))
  (if (`KismetSystemLibrary.IsValidClass` _currentitemclass)
    (`/Game/Blueprints/Inventory/Widgets/CraftMenu.UpdateDetailWindow` _craftmenu _currentitemclass))
  (return))

(fn `UpdateHotkeyForIndex`
  (params (index :type Integer))
  (if (`self.Showhotkeys?`)
    (for _array_element (`/Game/Blueprints/HUD/HUD.HotkeyWidgets` (`self.HUDWidget`))
      (bind _hotkeyslot (`/Game/Blueprints/HUD/Hotkey.HotkeySlot` _array_element))
      (if (and (not (`/Game/Blueprints/HUD/HotkeySlot.Empty?` _hotkeyslot)) (== (`/Game/Blueprints/HUD/HotkeySlot.InventoryIndex` _hotkeyslot) index))
        (`/Game/Blueprints/HUD/HotkeySlot.Update` _hotkeyslot)))
    (return)
    (else
      (return))))

(fn `UserConstructionScript`)