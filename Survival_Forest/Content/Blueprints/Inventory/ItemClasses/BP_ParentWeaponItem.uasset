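; Base item class for weapons in the inventory system, handling what happens when the weapon is used.
; Used calls EquipItem on the character held by the inventory reference, passing itself with the damage and attack radius from WeaponInfo as melee stats.
; If that call returns false, the item actor destroys itself.
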(event `self.Used`
  (bind (_weaponinfo_damage _weaponinfo_attackradius) (break `/Game/Blueprints/Inventory/Structures/S_WeaponInfo` (`self.WeaponInfo`)))
  (bind _success (`/Game/ThirdPersonBP/Blueprints/ThirdPersonCharacter.EquipItem` (`/Game/Blueprints/Inventory/BP_Inventory.CharRef` (`self.InventoryRef`)) self _weaponinfo_damage _weaponinfo_attackradius))
  (if (not _success)
    (`self.K2_DestroyActor`)))

(fn `UserConstructionScript`
  (`parent.UserConstructionScript`))