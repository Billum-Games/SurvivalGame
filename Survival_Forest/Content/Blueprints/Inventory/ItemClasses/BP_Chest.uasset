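; BP_Chest is an interactable chest that opens an item storage alongside the player's inventory.
; On BeginPlay it can roll starting loot from a data table, using per-row chance and amount range.
; The first interaction spawns a BP_Storage actor with that loot, which later interactions reuse, behind a DoOnce gate.
; Closing, also triggered when the character leaves the box while storage is open, hides the UI, restores walking and resets the gate.
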(event `self.ReceiveBeginPlay`
  (if (`self.GenerateStartItems?`)
    (`self.GenerateStartItems`)))

(event `OnInteract`
  (params (CharRefe :type "/Game/ThirdPersonBP/Blueprints/ThirdPersonCharacter Object Reference"))
  (bind _charref (`self.CharRef`))
  (bind _storageactorref (`self.StorageActorRef`))
  (bind _inventoryref (`/Game/ThirdPersonBP/Blueprints/ThirdPersonCharacter.InventoryRef` _charref))
  (`/Engine/EditorBlueprintResources/StandardMacros.DoOnce` false :!label _label
    (:`Completed`
      (set `self.CharRef` CharRefe)
      (`/Engine/EditorBlueprintResources/StandardMacros.IsValid` (`self.StorageActorRef`)
        (:`Is Valid`
          _)
        (:`Is Not Valid`
          (bind _returnvalue (`|SpawnActorFromClass` "/Game/Blueprints/Inventory/BP_Storage.BP_Storage_C" (`KismetMathLibrary.MakeTransform` (0.0 0.0 0.0)) "AlwaysSpawn" "OverrideRootScale" null (`self.AmountOfSlots`) (`self.CharRef`) (`self.SlotsPerRow`) self (`self.StartItems`) null))
          (set `self.StorageActorRef` _returnvalue)))
      (`/Game/Blueprints/Inventory/Widgets/Storage/StorageWidget.GenerateSlotWidgets` (`/Game/Blueprints/Inventory/BP_Storage.StorageWidget` _storageactorref) _storageactorref)
      (`/Game/Blueprints/Inventory/BP_Storage.ShowStorage` _storageactorref)
      (`/Game/Blueprints/Inventory/BP_Inventory.HideInventory` _inventoryref false)
      (`/Game/Blueprints/Inventory/BP_Inventory.ShowInventory` _inventoryref)
      (`MovementComponent.StopMovementImmediately` (`Character.CharacterMovement` _charref))
      (set `/Game/Blueprints/Inventory/BP_Inventory.InventoryOpen?` true _inventoryref))))

(event `OnStorageClosed`
  (bind _returnvalue (`GameplayStatics.GetPlayerController` 0))
  (bind _charref (`self.CharRef`))
  (bind _inventoryref (`/Game/ThirdPersonBP/Blueprints/ThirdPersonCharacter.InventoryRef` _charref))
  (`/Game/Blueprints/Inventory/BP_Storage.HideStorage` (`self.StorageActorRef`))
  (`CharacterMovementComponent.SetMovementMode` (`Character.CharacterMovement` _charref) "MOVE_Walking" 0)
  (if (`/Game/Blueprints/Inventory/BP_Inventory.InventoryOpen?` _inventoryref)
    (`/Game/Blueprints/Inventory/BP_Inventory.HideInventory` _inventoryref false)
    (set `PlayerController.bShowMouseCursor` false _returnvalue)
    (`WidgetBlueprintLibrary.SetInputMode_GameOnly` _returnvalue)
    (goto _label :!via `Reset`)
    (else
      (goto _label :!via `Reset`))))

(event `self.Box.OnComponentEndOverlap`
  (params (OverlappedComponent :type "PrimitiveComponent Object Reference") (OtherActor :type "Actor Object Reference") (OtherComp :type "PrimitiveComponent Object Reference") (OtherBodyIndex :type Integer))
  (bind _asthird_person_character (cast `/Game/ThirdPersonBP/Blueprints/ThirdPersonCharacter` OtherActor))
  (if (`/Game/Blueprints/Inventory/BP_Inventory.StorageOpen?` (`/Game/ThirdPersonBP/Blueprints/ThirdPersonCharacter.InventoryRef` _asthird_person_character))
    (`self.OnStorageClosed`)))

(fn `GenerateStartItems`
  (bind _outrownames (`DataTableFunctionLibrary.GetDataTableRowNames` "/Game/Blueprints/Inventory/Data_Tables/DTable_ChestStartItem.DTable_ChestStartItem"))
  (for _array_element _outrownames
    (bind _returnvalue (`|GetDataTableRow` "/Game/Blueprints/Inventory/Data_Tables/DTable_ChestStartItem.DTable_ChestStartItem" _array_element)
      (:`then`
        (if (and (<= (`KismetMathLibrary.RandomIntegerInRange` 1 100) (`.Chance_11_4410ABC644FAEA71FA76A58B094DAEBE` (break `/Game/Blueprints/Inventory/Structures/S_ChestContent` _returnvalue))) (`KismetSystemLibrary.IsValidClass` (break `/Game/Blueprints/Inventory/Structures/S_ChestContent` _returnvalue)))
          (`KismetArrayLibrary.Array_Add` (`self.StartItems`) (make `/Game/Blueprints/Inventory/Structures/S_InventorySlot` (break `/Game/Blueprints/Inventory/Structures/S_ChestContent` _returnvalue) (`KismetMathLibrary.RandomIntegerInRange` (`.MinAmount_9_018F049D493D467F3968CB9520BBF8B4` (break `/Game/Blueprints/Inventory/Structures/S_ChestContent` _returnvalue)) (`.MaxAmount_10_49F954F6498588FC09791A8FFB4617A7` (break `/Game/Blueprints/Inventory/Structures/S_ChestContent` _returnvalue)))))))))
  (return))

(fn `UserConstructionScript`)