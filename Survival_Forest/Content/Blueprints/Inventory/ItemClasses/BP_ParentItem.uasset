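; BP_ParentItem is a base pickup actor that the player can take into the inventory and use.
; Collision overlap enables input and starts a looping timer, never cleared here, that shows the HUD take prompt while the player's trace targets the item.
; Pressing E on the traced item adds it to the inventory, keeping any remainder, otherwise destroying it or flagging restoring items.
; Used removes one from the inventory and destroys the actor on success.
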(event `Used`
  (bind _success (`/Game/Blueprints/Inventory/BP_Inventory.RemoveItemAtIndex` (`self.InventoryRef`) (`self.Index`) 1))
  (if _success
    (`self.K2_DestroyActor`)))

(event `self.ReceiveBeginPlay`
  (bind _asthird_person_character (cast `/Game/ThirdPersonBP/Blueprints/ThirdPersonCharacter` (`GameplayStatics.GetPlayerCharacter` 0)))
  (set `self.PlayerRef` _asthird_person_character))

(event `TakeItem`
  (bind (_iteminfo_name _iteminfo_description _iteminfo_icon _iteminfo_can_be_used_ _iteminfo_howuses_text _iteminfo_canbestacked_ _iteminfo_category _iteminfo_subcategory _iteminfo_itemimportantparametr _iteminfo_isrestoring_) (break `/Game/Blueprints/Inventory/Structures/S_ItemInfo` (`self.ItemInfo`)))
  (bind _inventoryref (`/Game/ThirdPersonBP/Blueprints/ThirdPersonCharacter.InventoryRef` (`self.PlayerRef`)))
  (`/Engine/EditorBlueprintResources/StandardMacros.IsValid` _inventoryref
    (:`Is Valid`
      (bind (_success _rest) (`/Game/Blueprints/Inventory/BP_Inventory.AddItem` _inventoryref (`self.Item`) (`self.AmountOfItem`)))
      (if _success
        (if (> _rest 0)
          (set `self.AmountOfItem` _rest)
          (elif _iteminfo_isrestoring_
            (set `self.RestoreStarted` true)
            (set `self.AmountOfItem` 0)
            (else
              (`self.K2_DestroyActor`))))))))

(event `self.Collision.OnComponentBeginOverlap`
  (params (OverlappedComponent :type "PrimitiveComponent Object Reference") (OtherActor :type "Actor Object Reference") (OtherComp :type "PrimitiveComponent Object Reference") (OtherBodyIndex :type Integer) (bFromSweep :type Boolean) (SweepResult :type "HitResult Structure (by ref)"))
  (if (== OtherActor (`self.PlayerRef`))
    (set `self.CanInteract` true)
    (`self.EnableInput` (`GameplayStatics.GetPlayerController` 0))
    (`KismetSystemLibrary.K2_SetTimerDelegate` (delegate `TraceSelfDetected`) 0.1 (`self.CanInteract`))))

(event `self.Collision.OnComponentEndOverlap`
  (params (OverlappedComponent :type "PrimitiveComponent Object Reference") (OtherActor :type "Actor Object Reference") (OtherComp :type "PrimitiveComponent Object Reference") (OtherBodyIndex :type Integer))
  (if (== OtherActor (`self.PlayerRef`))
    (set `self.CanInteract` false)
    (`self.DisableInput` (`GameplayStatics.GetPlayerController` 0))))

(event `TraceSelfDetected`
  (bind _hudwidget (`/Game/Blueprints/Inventory/BP_Inventory.HUDWidget` (`/Game/ThirdPersonBP/Blueprints/ThirdPersonCharacter.InventoryRef` (`self.PlayerRef`))))
  (if (== (`/Game/ThirdPersonBP/Blueprints/ThirdPersonCharacter.TracingActor` (`self.PlayerRef`)) self)
    (`Widget.SetVisibility` (`/Game/Blueprints/HUD/HUD.TakeItemWidget` _hudwidget) "HitTestInvisible")
    (`/Game/Blueprints/HUD/HUD.Activate_WidgetTakeItem` _hudwidget (`self.ItemInfo`) (`self.AmountOfItem`))))

(event `Key|E`
  (params (Key :type "Key Structure"))
  (:`Pressed`
    (if (and (== (`/Game/ThirdPersonBP/Blueprints/ThirdPersonCharacter.TracingActor` (`self.PlayerRef`)) self) (`self.CanInteract`))
      (`self.TakeItem`))))

(fn `UserConstructionScript`)